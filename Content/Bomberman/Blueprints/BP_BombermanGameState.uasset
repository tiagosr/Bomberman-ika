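; BP_BombermanGameState is the game state Blueprint for a Bomberman game, tracking joined players and two action inputs.
; On BeginPlay it binds a player-joined handler that appends each new player to AllPlayers, with debug prints in both events.
; P1Action and P2Action input events set matching booleans while held.
; Tick loops over AllPlayers with an empty body.
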(event `self.ReceiveBeginPlay`
  (add `self.PlayerJoined` (delegate `On PlayerJoined`))
  (`KismetSystemLibrary.PrintString` "Init GameState"))

(event `On PlayerJoined` :!signature `self.PlayerJoined`
  (params (Player :type "/Game/Bomberman/Blueprints/BP_BombermanPawn Object Reference"))
  (`KismetArrayLibrary.Array_Append` (`self.All Players`) (`|MakeArray` Player))
  (`KismetSystemLibrary.PrintString` "Hello"))

(event `self.ReceiveTick`
  (params (DeltaSeconds :type "Float (single-precision)"))
  (for _ (`self.All Players`)
    _))

(event `InputAction|P1Action`
  (params (Key :type "Key Structure"))
  (:`Pressed`
    (set `self.P1Action` true))
  (:`Released`
    (set `self.P1Action` false)))

(event `InputAction|P2Action`
  (params (Key :type "Key Structure"))
  (:`Pressed`
    (set `self.P2Action` true))
  (:`Released`
    (set `self.P2Action` false)))

(fn `UserConstructionScript`)