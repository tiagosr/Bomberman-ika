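; Player pawn for a Bomberman game, colored by player index and supporting two local players.
; Tick feeds the indexed player's input into a controls event that rotates and moves the pawn with swept offsets, sliding along blocking surfaces.
; Releasing the action button spawns a bomb, limited by bomb count and a remote-control timer; exploded bombs leave the tracked list.
; Pickup events raise bomb power, speed or bomb count.
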(event `self.ReceiveBeginPlay`
  (add `self.PlayerControls` (delegate `On Player Controls`))
  (add `self.PowerUpPickup` (delegate `On Power-up Pickup`))
  (add `self.BombExploded` (delegate `BombExploded_Event`)))

(event `BombExploded_Event` :!signature `self.BombExploded`
  (params (Bomb :type "/Game/Bomberman/Blueprints/BP_BaseBomb Object Reference"))
  (bind _current_bombs (`self.Current Bombs`))
  (bind _returnvalue (`KismetArrayLibrary.Array_Find` _current_bombs Bomb))
  ;[1 1 1] Bomb reference removal
  (if (>= _returnvalue 0)
    (`KismetArrayLibrary.Array_Remove` _current_bombs _returnvalue)))

(event `On Power-up Pickup` :!signature `self.PowerUpPickup`
  (params (PickupType :type "/Game/Bomberman/Blueprints/EPickupTypes Enum" :default "NewEnumerator0"))
  ;[1 1 1] Powerup Buffs
  (switch `/Game/Bomberman/Blueprints/EPickupTypes` PickupType
    (:`NewEnumerator1`
      (set `self.Current Bomb Power` (+ (`self.Current Bomb Power`) 1)))
    (:`NewEnumerator2`
      (set `self.Movement Speed` (+ (`self.Movement Speed`) (`self.Movement Speed Increment`))))
    (:`NewEnumerator4`
      (set `self.Bomb Count` (+ (`self.Bomb Count`) 1)))))

(event `On Player Controls` :!signature `self.PlayerControls`
  (params (Amount :type "Vector Structure") (Action :type Boolean) (`Delta Seconds` :type "Float (double-precision)"))
  (bind _returnvalue (`KismetMathLibrary.MakeVector` Amount_X Amount_Y))
  (bind _returnvalue_2 (* _returnvalue (* `Delta Seconds` (`self.Movement Speed`))))
  (`|ExecutionSequence`
    (:`then_0`
      ;[1 1 1] Movement
      (if (> (`KismetMathLibrary.VSizeSquared` _returnvalue) 0.1)
        (`self.K2_SetActorRotation` (`KismetMathLibrary.FindLookAtRotation` (0.0 0.0 0.0) _returnvalue))
        (bind _sweephitresult (`self.K2_AddActorWorldOffset` _returnvalue_2 true))
        (bind (_bblockinghit _binitialoverlap _time _distance _location _impactpoint _normal) (`GameplayStatics.BreakHitResult` _sweephitresult))
        ;[1 1 1] Collision response
        (if _bblockinghit
          (`self.K2_AddActorWorldOffset` (* (`KismetMathLibrary.ProjectVectorOnToPlane` _returnvalue_2 (`KismetMathLibrary.Normal` (`KismetMathLibrary.MakeVector` (.x _normal) (.y _normal)))) (- 1.0 _time)) true))))
    (:`then_1`
      ;[1 1 1] Bomb button debounce
      (if (and (== Action false) (== (`self.Bomb Trigger Debounce`) true))
        ;[1 1 1] Bomb spawn control
        (if (> (`self.Remote Control Timer`) 0.0)
          _
          (elif (< (`KismetArrayLibrary.Array_Length` (`self.Current Bombs`)) (`self.Bomb Count`))
            ;[1 1 1] Creating bomb
            (bind _returnvalue_3 (`|SpawnActorFromClass` (`self.Current Bomb Type`) (`KismetMathLibrary.MakeTransform` (`self.K2_GetActorLocation`)) "AlwaysSpawn" "OverrideRootScale" self (`self.Current Bomb Time`) (`self.Current Bomb Power`) self))
            (`KismetArrayLibrary.Array_Add` (`self.Current Bombs`) _returnvalue_3)))))
    (:`then_2`
      (set `self.Bomb Trigger Debounce` Action))))

(event `self.ReceiveTick`
  (params (DeltaSeconds :type "Float (single-precision)"))
  ;[1 1 1] Remote control timer update
  (set `self.Remote Control Timer` (`KismetMathLibrary.FMax` (- (`self.Remote Control Timer`) DeltaSeconds)))
  ;[1 1 1] Input Handling (2 Players for now)
  (switch `int` (`self.Player Index`)
    (:`0`
      (`self.PlayerControls` (`KismetMathLibrary.MakeVector` (`self.GetInputAxisValue`) (`self.GetInputAxisValue`)) (`self.P1Action`) DeltaSeconds))
    (:`1`
      (`self.PlayerControls` (`KismetMathLibrary.MakeVector` (`self.GetInputAxisValue`) (`self.GetInputAxisValue`)) (`self.P2Action`) DeltaSeconds))))

(event `InputAction|P1Action`
  (params (Key :type "Key Structure"))
  ;[1 1 1] Input Handling (2 Players for now)
  (:`Pressed`
    (set `self.P1Action` true))
  (:`Released`
    (set `self.P1Action` false)))

(event `InputAction|P2Action`
  (params (Key :type "Key Structure"))
  ;[1 1 1] Input Handling (2 Players for now)
  (:`Pressed`
    (set `self.P2Action` true))
  (:`Released`
    (set `self.P2Action` false)))

(fn `UserConstructionScript`
  (bind _output (`|GetArrayItem` (`self.Player Colors`) (`self.Player Index`)))
  (if (`KismetSystemLibrary.IsValid` _output)
    (`PrimitiveComponent.SetMaterial` (`self.Cone`) 0 _output)))