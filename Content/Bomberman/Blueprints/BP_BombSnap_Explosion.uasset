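; Bomberman grid-cell Blueprint that displays bomb explosions and spreads them to linked neighbouring cells.
; The origin cell shows both X and Y visuals, activates its box and passes Power to all four neighbours.
; Directional events show one axis, enable query collision and relay onward in the same direction, decrementing Power until it runs out.
; A timer on each exploding cell then hides the visuals and disables collision.
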(event `self.ReceiveBeginPlay`
  (`self.Build Explosion` false)
  (add `self.Explode` (delegate `On Bomb Explode`))
  (add `self.ExplodeFromUp` (delegate `self.FExplodeFromUp`))
  (add `self.ExplodeFromDown` (delegate `self.FExplodeFromDown`))
  (add `self.ExplodeFromLeft` (delegate `self.FExplodeFromLeft`))
  (add `self.ExplodeFromRight` (delegate `self.FExplodeFromRight`)))

(event `On Bomb Explode` :!signature `self.Explode`
  (params (Power :type Integer))
  (bind _up (`self.Up`))
  (bind _down (`self.Down`))
  (bind _left (`self.Left`))
  (bind _right (`self.Right`))
  (`|ExecutionSequence`
    (:`then_0`
      (`SceneComponent.SetVisibility` (`self.Explosion_Y`) true false)
      (`SceneComponent.SetVisibility` (`self.Explosion_X`) true false)
      (`ActorComponent.SetActive` (`self.ExplosionBox`) true false)
      (`KismetSystemLibrary.K2_SetTimerDelegate` (delegate `On Explosion Finished`) (`self.Explosion Timer`)))
    (:`then_1`
      (if (`KismetSystemLibrary.IsValid` _up)
        (`self.FExplodeFromDown` _up Power)))
    (:`then_2`
      (if (`KismetSystemLibrary.IsValid` _down)
        (`self.FExplodeFromUp` _down Power)))
    (:`then_3`
      (if (`KismetSystemLibrary.IsValid` _left)
        (`self.FExplodeFromRight` _left Power)))
    (:`then_4`
      (if (`KismetSystemLibrary.IsValid` _right)
        (`self.FExplodeFromLeft` _right Power)))))

(event `On Explosion Finished`
  (`self.Explosion Time Expired`))

(event `self.FExplodeFromUp`
  (params (Power :type Integer))
  (bind _returnvalue (- Power 1))
  (bind _down (`self.Down`))
  (`self.Build Explosion` false true)
  (`KismetSystemLibrary.K2_SetTimerDelegate` (delegate `On Explosion Finished`) (`self.Explosion Timer`))
  (if (and (`KismetSystemLibrary.IsValid` _down) (>= _returnvalue 0))
    (`self.FExplodeFromUp` _down _returnvalue)))

(event `self.FExplodeFromDown`
  (params (Power :type Integer))
  (bind _returnvalue (- Power 1))
  (bind _up (`self.Up`))
  (`self.Build Explosion` false true)
  (`KismetSystemLibrary.K2_SetTimerDelegate` (delegate `On Explosion Finished`) (`self.Explosion Timer`))
  (if (and (`KismetSystemLibrary.IsValid` _up) (>= _returnvalue 0))
    (`self.FExplodeFromDown` _up _returnvalue)))

(event `self.FExplodeFromLeft`
  (params (Power :type Integer))
  (bind _returnvalue (- Power 1))
  (bind _right (`self.Right`))
  (`self.Build Explosion` true)
  (`KismetSystemLibrary.K2_SetTimerDelegate` (delegate `On Explosion Finished`) (`self.Explosion Timer`))
  (if (and (`KismetSystemLibrary.IsValid` _right) (>= _returnvalue 0))
    (`self.FExplodeFromLeft` _right _returnvalue)))

(event `self.FExplodeFromRight`
  (params (Power :type Integer))
  (bind _returnvalue (- Power 1))
  (bind _left (`self.Left`))
  (`self.Build Explosion` true)
  (`KismetSystemLibrary.K2_SetTimerDelegate` (delegate `On Explosion Finished`) (`self.Explosion Timer`))
  (if (and (`KismetSystemLibrary.IsValid` _left) (>= _returnvalue 0))
    (`self.FExplodeFromRight` _left _returnvalue)))

(fn `Build Explosion`
  (params (X :type Boolean) (Y :type Boolean))
  (bind _explosionbox (`self.ExplosionBox`))
  (`SceneComponent.SetVisibility` (`self.Explosion_Y`) Y false)
  (`SceneComponent.SetVisibility` (`self.Explosion_X`) X false)
  (if (or X Y)
    (`PrimitiveComponent.SetCollisionEnabled` _explosionbox "QueryOnly")
    (else
      (`PrimitiveComponent.SetCollisionEnabled` _explosionbox "NoCollision"))))

(fn `Explosion Time Expired`
  (`self.Build Explosion` false))

(fn `UserConstructionScript`)