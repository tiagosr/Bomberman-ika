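; StageGenerator is a Bomberman actor that builds the stage on BeginPlay as a centered grid of spawned blocks.
; Nested height and width loops position each cell from block size and offset.
; With StageBlocks empty, SelectSolidBlocks decides where BaseBlock spawns; otherwise each cell spawns its class from the flattened BlockTypes array.
; The BreakableBlock spawn is disconnected, and the edge-and-parity expression in SelectSolidBlocks is unused.
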(event `self.ReceiveBeginPlay`
  (bind _stage_height (`self.Stage Height`))
  (bind _stage_width (`self.Stage Width`))
  (for _index (range (+ _stage_height 1))
    (for _index_2 (range (+ _stage_width 1))
      (if (== (`KismetArrayLibrary.Array_Length` (`self.Stage Blocks`)) 0)
        (bind _returnvalue (`KismetMathLibrary.Min` _index_2 (- (`self.Stage Width`) _index_2)))
        (bind _returnvalue_2 (`KismetMathLibrary.Min` _index (- (`self.Stage Height`) _index)))
        (if (or (or (== _returnvalue 0) (== _returnvalue_2 0)) (or (== (mod _returnvalue 2) 0) (== (mod _returnvalue_2 2) 0)))
          (bind _returnvalue_3 (`KismetMathLibrary.Conv_VectorToTransform` (+ (`self.Block Offset`) (+ (* (`self.Block Size`) (`KismetMathLibrary.MakeVector` (`KismetMathLibrary.Conv_IntToDouble` _index_2) (`KismetMathLibrary.Conv_IntToDouble` _index))) (* (* (`self.Block Size`) (`KismetMathLibrary.MakeVector` (`KismetMathLibrary.Conv_IntToDouble` _stage_width) (`KismetMathLibrary.Conv_IntToDouble` _stage_height))) -0.5)))))
          (`|SpawnActorFromClass` "/Game/Bomberman/Objects/BaseBlock.BaseBlock_C" _returnvalue_3 "Undefined" "OverrideRootScale" null null))
        (else
          (`|SpawnActorFromClass` (`|GetArrayItem` (`self.Block Types`) (+ (* _stage_width _index) _index_2)) _returnvalue_3 "AlwaysSpawn" "OverrideRootScale"))))))