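; BP_Cameraman is the Bomberman camera actor that turns to keep the group of players in view without changing its position.
; On BeginPlay and every Tick, MoveCamera averages LookAtFocus with the locations of all valid Players, so the focus point acts as one extra weight in the centroid.
; It applies a look-at rotation toward that average, and StartPosition is saved at BeginPlay but not used in these graphs.
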(event `self.ReceiveBeginPlay`
  (set `self.StartPosition` (`self.K2_GetActorLocation`))
  (`self.MoveCamera`))

(event `self.ReceiveTick`
  (params (DeltaSeconds :type "Float (single-precision)"))
  (`self.MoveCamera`))

(fn `MoveCamera`
  (locals (LookAtInner :type "Vector Structure" :default (0.0 0.0 0.0)) (LookAtCount :type "Float (double-precision)" :default 1.0))
  (bind _output_get (set `local.LookAtInner` (`self.LookAtFocus`)))
  (set `local.LookAtCount` 1.0)
  (for _array_element (`self.Players`)
    (`/Engine/EditorBlueprintResources/StandardMacros.IsValid` _array_element
      (:`Is Valid`
        (set `local.LookAtInner` (+ (`self.K2_GetActorLocation` _array_element) (`local.LookAtInner`)))
        (`/Engine/EditorBlueprintResources/StandardMacros.IncrementFloat` (`local.LookAtCount`)))))
  (`self.K2_SetActorRotation` (`KismetMathLibrary.FindLookAtRotation` (`self.K2_GetActorLocation`) (/ _output_get (`local.LookAtCount`))))
  (return))

(fn `UserConstructionScript`)